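; BP_Gas is a colored Niagara gas cell that spreads and rises, layering by density (Densiter).
; Void detection traces both ways along Y and spawns copies with the same color and density into empty spaces.
; MoveGaz traces upward to climb, stop below obstacles or queue under other gas, sending denser gas downward.
; Tick interpolates toward Target, with timers and a resettable DoOnce pacing the steps.
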(event Custom|MoveGaz
  (bind _returnvalue (Transformation|GetActorLocation))
  ;[1 1 1] Calcul new position BP
  (Utilities|Time|SetTimerbyEvent (EventDispatchers|CreateEvent :!event Custom|reset) 0.2)
  (bind (_outhit _returnvalue_2) (Collision|LineTraceForObjects _returnvalue (+ _returnvalue "0.000000,0.000000,100.000000") (Utilities|Array|MakeArray "ObjectTypeQuery1" "ObjectTypeQuery2") true 0 "None"))
  (if _returnvalue_2
    (bind _asbp_gas (Utilities|Casting|CastToBP_Gas (.HitActor (Collision|BreakHitResult _outhit)))
      (:then
        (if (> (Variables|BP_Gas_C|GetDensiter _asbp_gas) (Variables|Default|GetDensiter))
          (Variables|Default|SetTarget (Transformation|GetActorLocation _asbp_gas))
          (Variables|BP_Gas_C|SetTarget _asbp_gas (- (Transformation|GetActorLocation) "0.000000,0.000000,100.000000"))
          (else
            (Variables|Default|SetTarget (- (Variables|BP_Gas_C|GetTarget _asbp_gas) "0.000000,0.000000,100.000000")))))
      (:CastFailed
        (Variables|Default|SetTarget (- (.Location (Collision|BreakHitResult _outhit)) "0.000000,0.000000,50.000000"))))
    (else
      (Variables|Default|SetTarget (+ (Variables|Default|GetTarget) "0.000000,0.000000,100.000000")))))

(event Custom|reset
  ;[1 1 1] Move BP
  (Utilities|FlowControl|DoOnce false) ; enters at Reset
)

(event Custom|VoidDetection
  (bind _returnvalue (Transformation|GetActorLocation))
  (bind _returnvalue_2 (Transformation|GetActorLocation))
  ;[1 1 1] Spawn New BP If Void Detected
  (Utilities|FlowControl|Sequence
    (:then_0
      (bind _returnvalue_3 (Collision|LineTraceForObjects (+ _returnvalue "0.000000,50.000000,0.000000") (+ _returnvalue "0.000000,100.000000,0.000000") (Utilities|Array|MakeArray "ObjectTypeQuery1" "ObjectTypeQuery2") false 0 "None"))
      (if (not _returnvalue_3)
        (bind _returnvalue_4 (Game|SpawnActorfromClass "BP_Gas_C" (Math|Transform|MakeTransform (+ (Transformation|GetActorLocation) "0.000000,100.000000,0.000000") "0, 0, 0" "1.000000,1.000000,1.000000") "DontSpawnIfColliding" "MultiplyWithRoot" 0 0))
        (CallFunction|InitNiagara _returnvalue_4 (Variables|Default|GetIn%20Value) (Variables|Default|GetDensiter))))
    (:then_1
      (bind _returnvalue_5 (Collision|LineTraceForObjects (+ _returnvalue_2 "0.000000,-50.000000,0.000000") (+ _returnvalue_2 "0.000000,-100.000000,0.000000") (Utilities|Array|MakeArray "ObjectTypeQuery1" "ObjectTypeQuery2") false 0 "None"))
      (if (not _returnvalue_5)
        (bind _returnvalue_6 (Game|SpawnActorfromClass "BP_Gas_C" (Math|Transform|MakeTransform (+ (Transformation|GetActorLocation) "0.000000,-100.000000,0.000000") "0, 0, 0" "1.000000,1.000000,1.000000") "DontSpawnIfColliding" "MultiplyWithRoot" 0 0))
        (CallFunction|InitNiagara _returnvalue_6 (Variables|Default|GetIn%20Value) (Variables|Default|GetDensiter))))))

(event Custom|InitNiagara
  (params (InValue :type Linear%20Color%20Structure%20%28by%20ref%29) (Densiter :type Float%20%28double-precision%29))
  ;[1 1 1] InitNewBPSpawn
  (bind _output_get (Variables|Default|SetIn%20Value InValue))
  (Niagara|SetNiagaraVariable(LinearColor) (Variables|Default|GetNiagara) "Color" _output_get)
  (Variables|Default|SetDensiter Densiter))

(event EventBeginPlay
  ;[1 1 1] Setup Target and play Void detection
  (Variables|Default|SetTarget (Transformation|GetActorLocation))
  (Utilities|Time|SetTimerbyEvent (EventDispatchers|CreateEvent :!event Custom|VoidDetection) 0.7))

(event Collision|EventActorBeginOverlap
  (params (OtherActor :type Actor%20Object%20Reference)))

(event EventTick
  (params (DeltaSeconds :type Float%20%28single-precision%29))
  (bind _returnvalue (Transformation|GetActorLocation))
  (bind _target (Variables|Default|GetTarget))
  (bind _interp_speed (Variables|Default|GetInterp%20Speed))
  (bind _returnvalue_2 (Math|Interpolation|VInterptoConstant _returnvalue _target DeltaSeconds _interp_speed))
  ;[1 1 1] Move BP
  (Transformation|SetActorLocation _returnvalue_2 false false)
  (if (Utilities|Operators|EqualEqual _returnvalue_2 (Variables|Default|GetTarget) 0.5)
    (Utilities|FlowControl|DoOnce false
      (:Completed
        (Utilities|Time|SetTimerbyEvent (EventDispatchers|CreateEvent :!event Custom|MoveGaz) 0.5)))))

(fn ConstructionScript
  (Niagara|SetNiagaraVariable(Vector3) (Variables|Default|GetNiagara) "ShapeSize" (Variables|/Script/Engine.BoxComponent|GetBoxExtent (Variables|Default|GetBox)))
  (Niagara|SetNiagaraVariable(LinearColor) (Variables|Default|GetNiagara) "Color" (Variables|Default|GetIn%20Value)))